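; BP_PacMan is the player-controlled Pac-Man that moves in four directions along world axes.
; On BeginPlay it adds the IAC_Move mapping context to the owning player's Enhanced Input subsystem.
; Each directional input action snaps the mesh to a fixed world rotation and adds movement input in the matching world direction.
; Only the Up action forces its movement input.
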(event `self.ReceiveBeginPlay`
  (bind _asplayer_controller (cast `PlayerController` (`self.GetController`)))
  (bind _returnvalue (pcsubsystem `EnhancedInputLocalPlayerSubsystem` _asplayer_controller))
  (`/Engine/EditorBlueprintResources/StandardMacros.IsValid` _returnvalue
    (:`Is Valid`
      (`EnhancedInputSubsystemInterface.AddMappingContext` _returnvalue "/Game/APacMan/Characters/PacMan/IAC_Move.IAC_Move" 0 (struct)))))

(event `EnhancedInput|/Game/APacMan/Characters/PacMan/IA_Up`
  (params (ActionValue :type Boolean) (ElapsedSeconds :type "Float (double-precision)") (TriggeredSeconds :type "Float (double-precision)") (InputAction :type "InputAction Object Reference" :default "/Game/APacMan/Characters/PacMan/IA_Up.IA_Up"))
  (:`Triggered`
    (`SceneComponent.K2_SetWorldRotation` :`self` (`self.Mesh`))
    (`self.AddMovementInput` (`KismetMathLibrary.Vector_Forward`) 1.0 true)))

(event `EnhancedInput|/Game/APacMan/Characters/PacMan/IA_Down`
  (params (ActionValue :type Boolean) (ElapsedSeconds :type "Float (double-precision)") (TriggeredSeconds :type "Float (double-precision)") (InputAction :type "InputAction Object Reference" :default "/Game/APacMan/Characters/PacMan/IA_Down.IA_Down"))
  (:`Triggered`
    (`SceneComponent.K2_SetWorldRotation` (`self.Mesh`) (struct :`Yaw` 180.0) false false)
    (`self.AddMovementInput` (`KismetMathLibrary.Vector_Backward`))))

(event `EnhancedInput|/Game/APacMan/Characters/PacMan/IA_Left`
  (params (ActionValue :type Boolean) (ElapsedSeconds :type "Float (double-precision)") (TriggeredSeconds :type "Float (double-precision)") (InputAction :type "InputAction Object Reference" :default "/Game/APacMan/Characters/PacMan/IA_Left.IA_Left"))
  (:`Triggered`
    (`SceneComponent.K2_SetWorldRotation` (`self.Mesh`) (struct :`Yaw` 270.0) false false)
    (`self.AddMovementInput` (`KismetMathLibrary.Vector_Left`))))

(event `EnhancedInput|/Game/APacMan/Characters/PacMan/IA_Right`
  (params (ActionValue :type Boolean) (ElapsedSeconds :type "Float (double-precision)") (TriggeredSeconds :type "Float (double-precision)") (InputAction :type "InputAction Object Reference" :default "/Game/APacMan/Characters/PacMan/IA_Right.IA_Right"))
  (:`Triggered`
    (`SceneComponent.K2_SetWorldRotation` (`self.Mesh`) (struct :`Yaw` 90.0) false false)
    (`self.AddMovementInput` (`KismetMathLibrary.Vector_Right`))))

(fn `UserConstructionScript`)