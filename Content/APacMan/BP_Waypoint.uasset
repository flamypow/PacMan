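; Maze waypoint actor for a Pac-Man style game that picks a new moving direction for ghosts passing through it.
; The construction script converts the AllowedDirection map into a set of open directions and hides the indicator components of blocked ones.
; On sphere overlap, a ghost gets a random open direction, excluding a reversal.
; The ghost's IsOnWaypoint flag blocks repeat picks until the overlap ends.
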(event `self.Sphere.OnComponentBeginOverlap`
  (params (OverlappedComponent :type "PrimitiveComponent Object Reference") (OtherActor :type "Actor Object Reference") (OtherComp :type "PrimitiveComponent Object Reference") (OtherBodyIndex :type Integer) (bFromSweep :type Boolean) (SweepResult :type "HitResult Structure (by ref)"))
  (bind _asbp_ghost (cast `/Game/APacMan/Characters/Ghost/BP_Ghost` OtherActor))
  (if (== (`/Game/APacMan/Characters/Ghost/BP_Ghost.isOnWaypoint` _asbp_ghost) false)
    (set `/Game/APacMan/Characters/Ghost/BP_Ghost.isOnWaypoint` true _asbp_ghost)
    (set `self.TempAllowedDirection` (`self.AllowedDirectionVer2`))
    (`BlueprintSetLibrary.Set_Remove` (`self.TempAllowedDirection`) (`/Game/APacMan/FunctionLibrary.OppositeDirection` (`/Game/APacMan/Characters/Ghost/BP_Ghost.MovingDirection` _asbp_ghost)))
    (bind _result (`BlueprintSetLibrary.Set_ToArray` (`self.TempAllowedDirection`)))
    (set `/Game/APacMan/Characters/Ghost/BP_Ghost.MovingDirection` (`|GetArrayItem` _result (`KismetMathLibrary.RandomInteger` (`KismetArrayLibrary.Array_Length` _result))) _asbp_ghost)))

(event `self.Sphere.OnComponentEndOverlap`
  (params (OverlappedComponent :type "PrimitiveComponent Object Reference") (OtherActor :type "Actor Object Reference") (OtherComp :type "PrimitiveComponent Object Reference") (OtherBodyIndex :type Integer))
  (bind _asbp_ghost (cast `/Game/APacMan/Characters/Ghost/BP_Ghost` OtherActor))
  (set `/Game/APacMan/Characters/Ghost/BP_Ghost.isOnWaypoint` false _asbp_ghost))

(fn `UserConstructionScript`
  (bind _enumvalue (foreach `/Game/APacMan/E_Directions` false)
    (:`LoopBody`
      (switch `/Game/APacMan/E_Directions` _enumvalue
        (:`NewEnumerator0`
          (bind _returnvalue (== (`BlueprintMapLibrary.Map_Find` (`self.AllowedDirection`) _enumvalue) false))
          (if _returnvalue
            (`SceneComponent.SetVisibility` (`self.up`) false false)
            (else
              (`BlueprintSetLibrary.Set_Add` (`self.AllowedDirectionVer2`) "NewEnumerator0"))))
        (:`NewEnumerator1`
          (if _returnvalue
            (`SceneComponent.SetVisibility` (`self.Down`) false false)
            (else
              (`BlueprintSetLibrary.Set_Add` (`self.AllowedDirectionVer2`) "NewEnumerator1"))))
        (:`NewEnumerator2`
          (if _returnvalue
            (`SceneComponent.SetVisibility` (`self.Left`) false false)
            (else
              (`BlueprintSetLibrary.Set_Add` (`self.AllowedDirectionVer2`) "NewEnumerator2"))))
        (:`NewEnumerator3`
          (if _returnvalue
            (`SceneComponent.SetVisibility` (`self.Right`) false false)
            (else
              (`BlueprintSetLibrary.Set_Add` (`self.AllowedDirectionVer2`) "NewEnumerator3"))))))))