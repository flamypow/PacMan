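; BP_ScoreManager is an actor that tracks pellet collection in a Pac-Man game and handles level completion.
; Each PelletCollected call increments the player's count and compares it to the level's pellet total.
; On a match it prints a win message, raises InsMovespeed on GI_PacMan by DifficultyIncrease, then opens ThirdPersonMap after a delay.
; Keeping that speed in the game instance carries the difficulty increase across the level load.
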(event `PelletCollected`
  (bind _result (`/Engine/EditorBlueprintResources/StandardMacros.IncrementInt` (`self.PlayerPellets`))
    (:`  `
      (set `self.PlayerPellets` _result)
      (if (== (`self.PlayerPellets`) (`self.TotalPelletsInLevel`))
        (`KismetSystemLibrary.PrintString` "You Beat the level, Loading the next one")
        (bind _asgi_pac_man (cast `/Game/APacMan/GI_PacMan` (`GameplayStatics.GetGameInstance`)))
        (set `/Game/APacMan/GI_PacMan.Ins Movespeed` (+ (`/Game/APacMan/GI_PacMan.Ins Movespeed` _asgi_pac_man) (`self.DifficultyIncrease`)) _asgi_pac_man)
        (`KismetSystemLibrary.Delay` 5.0)
        (`GameplayStatics.OpenLevel` "ThirdPersonMap")))))

(fn `UserConstructionScript`)